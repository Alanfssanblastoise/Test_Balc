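; Player Blueprint for the Door and Key System that handles picking up keys, coins and powerups on collision overlap.
; It switches on pickable type, stores the tutorial key and coins in ACDAKSInventory and refreshes the UI_Manager widget.
; Coin sounds play at random offsets around the player, with coin and powerup pitch rising with coin count.
; Powerups only print their type and get destroyed, while the key's destroy call is unconnected.
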(event `self.ReceiveBeginPlay`
  (bind _returnvalue (`GameplayStatics.GetActorOfClass` "/Game/Logic/DoorAndKeySystem/UI_Manager0.UI_Manager0_C"))
  (set `self.UI_Widget` (`/Game/Logic/DoorAndKeySystem/UI_Manager0.Widget` _returnvalue)))

(event `self.CollisionComponent.OnComponentBeginOverlap`
  (params (OverlappedComponent :type "PrimitiveComponent Object Reference") (OtherActor :type "Actor Object Reference") (OtherComp :type "PrimitiveComponent Object Reference") (OtherBodyIndex :type Integer) (bFromSweep :type Boolean) (SweepResult :type "HitResult Structure (by ref)"))
  (bind _asbp_pickable (cast `/Game/Logic/DoorAndKeySystem/BP_Pickable` OtherActor))
  (switch `/Game/Logic/DoorAndKeySystem/E_PickableType` (`/Game/Logic/DoorAndKeySystem/BP_Pickable.PickableType` _asbp_pickable)
    (:`NewEnumerator0`
      (bind _asbp_key (cast `/Game/Logic/DoorAndKeySystem/BP_Key` _asbp_pickable)
        (:`then`
          (`/Engine/EditorBlueprintResources/StandardMacros.IsValid` _asbp_key
            (:`Is Valid`
              (if (== (`/Game/Logic/DoorAndKeySystem/BP_Key.KeyType` _asbp_key) 0)
                (bind _output_get (set `/Game/Logic/DoorAndKeySystem/AC_DAKS_Inventory.bTutorialKey` true (`self.AC_DAKS_Inventory`)))
                (`/Game/Logic/DoorAndKeySystem/WBP_DAKS.Refresh_Keys` (`self.UI_Widget`) _output_get)
                (`GameplayStatics.PlaySoundAtLocation` "/Game/Logic/DoorAndKeySystem/SFX_PickUpKey.SFX_PickUpKey" (0.0 0.0 0.0) (struct) 1.0 1.0 0.0 null null null null)
                (else
                  (`KismetSystemLibrary.LogString` "picked wrong Key"))))
            (:`Is Not Valid`
              (`KismetSystemLibrary.LogString` "invalid Key"))))
        (:`CastFailed`
          (`KismetSystemLibrary.LogString` "Key cast failed"))))
    (:`NewEnumerator1`
      (bind _asbp_coin (cast `/Game/Logic/DoorAndKeySystem/BP_Coin` _asbp_pickable)
        (:`then`
          (`/Engine/EditorBlueprintResources/StandardMacros.IsValid` _asbp_coin
            (:`Is Valid`
              (bind _output_get_2 (set `/Game/Logic/DoorAndKeySystem/AC_DAKS_Inventory.CoinsAmmount` (+ (`/Game/Logic/DoorAndKeySystem/BP_Coin.Value` _asbp_coin) (`/Game/Logic/DoorAndKeySystem/AC_DAKS_Inventory.CoinsAmmount` (`self.AC_DAKS_Inventory`))) (`self.AC_DAKS_Inventory`)))
              (`/Game/Logic/DoorAndKeySystem/WBP_DAKS.Refresh_Coins` (`self.UI_Widget`) _output_get_2)
              (`GameplayStatics.PlaySoundAtLocation` "/Game/Logic/DoorAndKeySystem/SFX_PickUpCoin.SFX_PickUpCoin" (+ (`self.K2_GetActorLocation`) (`KismetMathLibrary.MakeVector` (`KismetMathLibrary.RandomFloatInRange` -100.0 100.0) (`KismetMathLibrary.RandomFloatInRange` -100.0 100.0) (`KismetMathLibrary.RandomFloatInRange` -100.0 100.0))) (struct) 1.0 (+ (* (`KismetMathLibrary.Conv_IntToDouble` _output_get_2) 0.05) 1.0) 0.0 "/Game/Logic/DoorAndKeySystem/SA_Test.SA_Test" null null null)
              (`self.K2_DestroyActor` _asbp_coin))
            (:`Is Not Valid`
              (`KismetSystemLibrary.LogString` "invalid Coin"))))
        (:`CastFailed`
          (`KismetSystemLibrary.LogString` "Coin cast failed"))))
    (:`NewEnumerator2`
      (bind _asbp_powerup (cast `/Game/Logic/DoorAndKeySystem/BP_Powerup` _asbp_pickable)
        (:`then`
          (`/Engine/EditorBlueprintResources/StandardMacros.IsValid` _asbp_powerup
            (:`Is Valid`
              (`KismetSystemLibrary.PrintString` (`KismetStringLibrary.Concat_StrStr` "Powerup picked: " (`|GetEnumeratorNameAsString` (`/Game/Logic/DoorAndKeySystem/BP_Powerup.PowerupType` _asbp_powerup))))
              (`GameplayStatics.PlaySoundAtLocation` "/Game/Logic/DoorAndKeySystem/SFX_Powerup.SFX_Powerup" (`self.K2_GetActorLocation` _asbp_powerup) (struct) 1.0 (+ (/ (`KismetMathLibrary.Conv_IntToDouble` (`/Game/Logic/DoorAndKeySystem/AC_DAKS_Inventory.CoinsAmmount` (`self.AC_DAKS_Inventory`))) 10.0) 1.0) 0.0 null null null null)
              (`self.K2_DestroyActor` _asbp_powerup))
            (:`Is Not Valid`
              (`KismetSystemLibrary.LogString` "invalid Powerup"))))
        (:`CastFailed`
          (`KismetSystemLibrary.LogString` "Powerup cast failed"))))))

(fn `UserConstructionScript`)