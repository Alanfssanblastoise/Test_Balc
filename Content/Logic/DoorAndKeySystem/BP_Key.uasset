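; BP_Key is a key pickup in the door and key system, with variants for the tutorial, level 1 and level 2.
; Its construction script picks KeyMesh from the KeyType enum and sets PickableType to a fixed enum value before calling the parent construction script.
; The event graph holds only disabled default events, so the Blueprint adds no runtime logic of its own.
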(fn `UserConstructionScript`
  (set `self.KeyMesh` (select `/Game/Logic/DoorAndKeySystem/E_KeyType` (`self.KeyType`) :`NewEnumerator0` (`self.Tutorial`) :`NewEnumerator1` (`self.Lvl 1`) :`NewEnumerator2` (`self.Lvl 2`)))
  (set `self.PickableType` "NewEnumerator0")
  (`parent.UserConstructionScript`))